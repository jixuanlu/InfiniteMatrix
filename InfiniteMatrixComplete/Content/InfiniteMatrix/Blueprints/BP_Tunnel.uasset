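; BP_Tunnel is an endless-tunnel segment with a rotating holed wall, health kit and enemy.
; Its trigger zone adds score and asks TunnelSpawner for the next segment.
; Wall and enemy overlaps shake the camera and flash red on begin, then damage the player on end; shot enemies award score.
; Uncalled-here functions randomize wall, kit and enemy; kit pickup or spawn lifespans destroy the whole segment, not just the component.
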(event OnComponentBeginOverlap(TriggerZone)
  (params (OverlappedComponent :type Primitive%20Component%20Object%20Reference) (OtherActor :type Actor%20Object%20Reference) (OtherComp :type Primitive%20Component%20Object%20Reference) (OtherBodyIndex :type Integer) (bFromSweep :type Boolean) (SweepResult :type Hit%20Result%20Structure%20%28by%20ref%29))
  (bind _asbp_player (Utilities|Casting|CastToBP_Player OtherActor))
  (Default|IncrementScore _asbp_player)
  (Default|SpawnTunnelatSpawnPoint (Variables|Default|GetTunnelSpawner)))

(event OnComponentEndOverlap(WallMesh)
  (params (OverlappedComponent :type Primitive%20Component%20Object%20Reference) (OtherActor :type Actor%20Object%20Reference) (OtherComp :type Primitive%20Component%20Object%20Reference) (OtherBodyIndex :type Integer))
  (bind _asbp_player (Utilities|Casting|CastToBP_Player OtherActor))
  (Default|DecrementScore _asbp_player)
  (Variables|/Game/InfiniteMatrix/Blueprints/BP_Player.BP_Player_C|SetCurrentHealth _asbp_player (- (Variables|/Game/InfiniteMatrix/Blueprints/BP_Player.BP_Player_C|GetCurrentHealth _asbp_player) 2e+01))
  (if (<= (Variables|/Game/InfiniteMatrix/Blueprints/BP_Player.BP_Player_C|GetCurrentHealth _asbp_player) (Variables|/Game/InfiniteMatrix/Blueprints/BP_Player.BP_Player_C|GetMinHealth _asbp_player))
    (Variables|/Game/InfiniteMatrix/Blueprints/BP_Player.BP_Player_C|SetIsDead _asbp_player true)
    (Default|DisplayRestart _asbp_player)
    (else
      (Variables|/Game/InfiniteMatrix/Blueprints/BP_Player.BP_Player_C|SetIsDead _asbp_player false))))

(event OnComponentBeginOverlap(Enemy)
  (params (OverlappedComponent :type Primitive%20Component%20Object%20Reference) (OtherActor :type Actor%20Object%20Reference) (OtherComp :type Primitive%20Component%20Object%20Reference) (OtherBodyIndex :type Integer) (bFromSweep :type Boolean) (SweepResult :type Hit%20Result%20Structure%20%28by%20ref%29))
  (bind _asbp_player (Utilities|Casting|CastToBP_Player OtherActor)
    (:then
      ;[1 1 1] Shake camera when gets hurt
      (Camera|PlayWorldCameraShake "/Game/InfiniteMatrix/Blueprints/Shack_Camera.Shack_Camera_C" (Transformation|GetActorLocation _asbp_player) 0.0 1e+02)
      ;[1 1 1] Flash red when gets hurt
      (bind _returnvalue (UserInterface|CreateWidget "/Game/InfiniteMatrix/UI/WBP_Hurt.WBP_Hurt_C"))
      (UserInterface|Viewport|AddtoViewport _returnvalue 0)
      (Components|DestroyComponent (Variables|Default|GetEnemy)))
    (:CastFailed
      (Components|DestroyComponent (Variables|Default|GetEnemy))
      (bind _asbp_player_2 (Utilities|Casting|CastToBP_Player (Game|Player|GetPlayerPawn 0)))
      (Default|IncrementScore _asbp_player_2)
      (bind _asbp_projectile (Utilities|Casting|CastToBP_Projectile OtherActor))
      (Actor|DestroyActor _asbp_projectile))))

(event OnComponentEndOverlap(HealthKit)
  (params (OverlappedComponent :type Primitive%20Component%20Object%20Reference) (OtherActor :type Actor%20Object%20Reference) (OtherComp :type Primitive%20Component%20Object%20Reference) (OtherBodyIndex :type Integer))
  (bind _asbp_player (Utilities|Casting|CastToBP_Player OtherActor)
    (:then
      (if (not (>= (Variables|/Game/InfiniteMatrix/Blueprints/BP_Player.BP_Player_C|GetCurrentHealth _asbp_player) (Variables|/Game/InfiniteMatrix/Blueprints/BP_Player.BP_Player_C|GetMaxHealth _asbp_player)))
        (Variables|/Game/InfiniteMatrix/Blueprints/BP_Player.BP_Player_C|SetCurrentHealth _asbp_player (+ (Variables|/Game/InfiniteMatrix/Blueprints/BP_Player.BP_Player_C|GetCurrentHealth _asbp_player) 1e+01))
        (Actor|DestroyActor)))
    (:CastFailed
      (bind _asbp_projectile (Utilities|Casting|CastToBP_Projectile OtherActor))
      (Actor|DestroyActor _asbp_projectile))))

(event OnComponentEndOverlap(Enemy)
  (params (OverlappedComponent :type Primitive%20Component%20Object%20Reference) (OtherActor :type Actor%20Object%20Reference) (OtherComp :type Primitive%20Component%20Object%20Reference) (OtherBodyIndex :type Integer))
  (bind _asbp_player (Utilities|Casting|CastToBP_Player OtherActor))
  (Variables|/Game/InfiniteMatrix/Blueprints/BP_Player.BP_Player_C|SetCurrentHealth _asbp_player (- (Variables|/Game/InfiniteMatrix/Blueprints/BP_Player.BP_Player_C|GetCurrentHealth _asbp_player) 2e+01))
  (if (<= (Variables|/Game/InfiniteMatrix/Blueprints/BP_Player.BP_Player_C|GetCurrentHealth _asbp_player) (Variables|/Game/InfiniteMatrix/Blueprints/BP_Player.BP_Player_C|GetMinHealth _asbp_player))
    (Variables|/Game/InfiniteMatrix/Blueprints/BP_Player.BP_Player_C|SetIsDead _asbp_player true)
    (Default|DisplayRestart _asbp_player)
    (else
      (Variables|/Game/InfiniteMatrix/Blueprints/BP_Player.BP_Player_C|SetIsDead _asbp_player false))))

(event OnComponentBeginOverlap(WallMesh)
  (params (OverlappedComponent :type Primitive%20Component%20Object%20Reference) (OtherActor :type Actor%20Object%20Reference) (OtherComp :type Primitive%20Component%20Object%20Reference) (OtherBodyIndex :type Integer) (bFromSweep :type Boolean) (SweepResult :type Hit%20Result%20Structure%20%28by%20ref%29))
  (bind _asbp_player (Utilities|Casting|CastToBP_Player OtherActor)
    (:then
      ;[1 1 1] Shake camera when gets hurt
      (Camera|PlayWorldCameraShake "/Game/InfiniteMatrix/Blueprints/Shack_Camera.Shack_Camera_C" (Transformation|GetActorLocation _asbp_player) 0.0 1e+02)
      ;[1 1 1] Flash red when gets hurt
      (bind _returnvalue (UserInterface|CreateWidget "/Game/InfiniteMatrix/UI/WBP_Hurt.WBP_Hurt_C"))
      (UserInterface|Viewport|AddtoViewport _returnvalue 0))
    (:CastFailed
      (bind _asbp_projectile (Utilities|Casting|CastToBP_Projectile OtherActor))
      (Actor|DestroyActor _asbp_projectile))))

(event EventBeginPlay)

(event EventTick
  (params (DeltaSeconds :type Float%20%28single-precision%29))
  (Transformation|AddLocalRotation (Variables|Default|GetWallMesh) (Math|Rotator|MakeRotator (* DeltaSeconds (Variables|Default|GetRotateSpeed)) 0.0 0.0) false false)
  (Transformation|AddLocalRotation (Variables|Default|GetHealthKit) (Math|Rotator|MakeRotator 0.0 0.0 (* DeltaSeconds (Variables|Default|GetRotateSpeed) 1e+01)) false false))

(fn ConstructionScript)

(fn RandomizeWall
  (Components|StaticMesh|SetStaticMesh (Variables|Default|GetWallMesh) (Utilities|Select :Index (Math|Random|RandomIntegerinRange 0 3) :Option%200 "/Game/InfiniteMatrix/Meshes/SM_Hole_01.SM_Hole_01" :Option%201 "/Game/InfiniteMatrix/Meshes/SM_Hole_02.SM_Hole_02" :Option%202 "/Game/InfiniteMatrix/Meshes/SM_Hole_03.SM_Hole_03" :Option%203 "/Game/InfiniteMatrix/Meshes/SM_Hole_04.SM_Hole_04"))
  (Transformation|AddLocalRotation (Variables|Default|GetWallMesh) (Math|Rotator|MakeRotator (Math|Random|RandomFloatinRange 0.0 3.6e+02) 0.0 0.0) false false))

(fn RandomizedKit
  (Transformation|AddLocalOffset (Variables|Default|GetHealthKit) (Math|Vector|MakeVector (Math|Random|RandomFloatinRange 2e+02 2.3e+03) (Math|Random|RandomFloatinRange -2.8e+02 2.8e+02) (Math|Random|RandomFloatinRange -2.8e+02 2.8e+02)) false false)
  (if (== (Math|Random|RandomIntegerinRange 1 4) 4)
    (Components|StaticMesh|SetStaticMesh (Variables|Default|GetHealthKit) "/Game/InfiniteMatrix/Meshes/Health_Kit.Health_Kit")
    (Actor|SetLifeSpan (Components|GetOwner (Variables|Default|GetHealthKit)) 1e+01)
    (else
      (Components|StaticMesh|SetStaticMesh (Variables|Default|GetHealthKit) 0))))

(fn RandomizeEnemy
  (Transformation|AddLocalOffset (Variables|Default|GetEnemy) (Math|Vector|MakeVector (Math|Random|RandomFloatinRange 2e+02 2.3e+03) (Math|Random|RandomFloatinRange -2.8e+02 2.8e+02) (Math|Random|RandomFloatinRange -2.8e+02 2.8e+02)) false false)
  (if (== (Math|Random|RandomIntegerinRange 1 3) 3)
    (Components|StaticMesh|SetStaticMesh (Variables|Default|GetEnemy) "/Game/InfiniteMatrix/Meshes/Enemy.Enemy")
    (Actor|SetLifeSpan (Components|GetOwner (Variables|Default|GetEnemy)) 1e+01)
    (else
      (Components|StaticMesh|SetStaticMesh (Variables|Default|GetEnemy) 0))))