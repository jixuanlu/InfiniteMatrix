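; BP_Projectile is a projectile actor that flies forward along its local X axis and speeds up as the player's score rises.
; Each Tick casts the player pawn to BP_Player, adds a Score-scaled bonus to ProjectileSpeed, and applies a swept, delta-time-scaled local offset.
; The sphere overlap event is empty, and the DestroyComponent call is never run, so the graph contains no hit handling.
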(event OnComponentBeginOverlap(Sphere)
  (params (OverlappedComponent :type Primitive%20Component%20Object%20Reference) (OtherActor :type Actor%20Object%20Reference) (OtherComp :type Primitive%20Component%20Object%20Reference) (OtherBodyIndex :type Integer) (bFromSweep :type Boolean) (SweepResult :type Hit%20Result%20Structure%20%28by%20ref%29)))

(event EventBeginPlay)

(event EventTick
  (params (DeltaSeconds :type Float%20%28single-precision%29))
  (bind _asbp_player (Utilities|Casting|CastToBP_Player (Game|Player|GetPlayerPawn 0)))
  (Transformation|AddActorLocalOffset (Math|Vector|MakeVector (* (+ (Variables|Default|GetProjectileSpeed) (* (Math|Conversions|ToFloat(Integer) (Variables|/Game/InfiniteMatrix/Blueprints/BP_Player.BP_Player_C|GetScore _asbp_player)) 5e+01)) DeltaSeconds) 0.0 0.0) true false))

(fn ConstructionScript)